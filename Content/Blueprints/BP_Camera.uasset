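; Player camera Blueprint for a city-building game that acts as the bridge between game events and the UI.
; Each event casts a stored widget instance, some held on Grid, to its UI class and forwards the update.
; These cover resources, research, parliament, diplomacy, map, logs, info panels and warnings.
; BeginPlay keeps the player controller fully ticking while paused, and UnlockAchievement caches achievements before writing progress.
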(event `self.ReceiveBeginPlay`
  (set `PlayerController.bShouldPerformFullTickWhenPaused` true (`GameplayStatics.GetPlayerController` 0)))

(event `self.UpdateDisplayName`
  (bind _asinteract_ui (cast `/Game/Blueprints/UI/Interactions/InteractUI` (`WidgetComponent.GetWidget` (`self.WidgetComponent`))))
  (`/Game/Blueprints/UI/Interactions/InteractUI.SetBuildingDisplayName` _asinteract_ui))

(event `self.SetInteractableText`
  (params (Actor :type "Actor Object Reference") (Instance :type Integer))
  (bind _asinteract_ui (cast `/Game/Blueprints/UI/Interactions/InteractUI` (`WidgetComponent.GetWidget` (`self.WidgetComponent`))))
  (`/Game/Blueprints/UI/Interactions/InteractUI.SetDisplayText` _asinteract_ui Actor Instance))

(event `self.UpdateHealthIssues`
  (bind _asinteract_ui (cast `/Game/Blueprints/UI/Interactions/InteractUI` (`WidgetComponent.GetWidget` (`self.WidgetComponent`))))
  (`/Game/Blueprints/UI/Interactions/InteractUI.CallHealthIssues` _asinteract_ui))

(event `self.UpdateDayText`
  (bind _asmain_ui (cast `/Game/Blueprints/UI/MainUI` (`self.BuildUIInstance`)))
  (`/Game/Blueprints/UI/MainUI.SetDayText` _asmain_ui))

(event `self.UpdateResourceText`
  (params (Category :type String))
  (bind _asmain_ui (cast `/Game/Blueprints/UI/MainUI` (`self.BuildUIInstance`)))
  (`/Game/Blueprints/UI/MainUI.SetResourceText` _asmain_ui Category))

(event `self.UpdateResourceCapacityText`
  (params (Category :type String))
  (bind _asmain_ui (cast `/Game/Blueprints/UI/MainUI` (`self.BuildUIInstance`)))
  (`/Game/Blueprints/UI/MainUI.SetCapacityText` _asmain_ui Category))

(event `self.UpdateUI`
  (params (Happiness :type "Float (single-precision)") (Rebels :type "Float (single-precision)"))
  (bind _asmain_ui (cast `/Game/Blueprints/UI/MainUI` (`self.BuildUIInstance`)))
  (`/Game/Blueprints/UI/MainUI.SetOverallInfoUI` _asmain_ui Happiness Rebels))

(event `self.SetSeedVisibility`
  (params (bVisible :type Boolean))
  (bind _asmain_ui (cast `/Game/Blueprints/UI/MainUI` (`self.BuildUIInstance`)))
  (`/Game/Blueprints/UI/MainUI.SetSeedVisibility` _asmain_ui bVisible))

(event `self.UpdateTrends`
  (bind _asmain_ui (cast `/Game/Blueprints/UI/MainUI` (`self.BuildUIInstance`)))
  (`/Game/Blueprints/UI/MainUI.SetTrendText` _asmain_ui))

(event `self.UpdateSpeedUI`
  (params (Speed :type "Float (single-precision)"))
  (bind _asmain_ui (cast `/Game/Blueprints/UI/MainUI` (`self.BuildUIInstance`)))
  (`/Game/Blueprints/UI/MainUI.SetSpeedUI` _asmain_ui Speed))

(event `self.SetCurrentResearchUI`
  (bind _asmain_ui (cast `/Game/Blueprints/UI/MainUI` (`self.BuildUIInstance`)))
  (`/Game/Blueprints/UI/MainUI.DisplayResearch` _asmain_ui)
  (bind _asresearch_ui (cast `/Game/Blueprints/UI/Research/ResearchUI` (`self.ResearchUIInstance`)))
  (`/Game/Blueprints/UI/Research/ResearchUI.UpdateResearchUI` _asresearch_ui))

(event `self.RemoveResearchUI`
  (params (QueueIndex :type Integer))
  (bind _asresearch_ui (cast `/Game/Blueprints/UI/Research/ResearchUI` (`self.ResearchUIInstance`)))
  (`/Game/Blueprints/UI/Research/ResearchUI.RemoveResearchUI` _asresearch_ui QueueIndex))

(event `self.DisplayEvent`
  (params (Descriptor :type String) (Event :type String))
  (bind _asevent_ui (cast `/Game/Blueprints/UI/EventUI` (`self.EventUIInstance`)))
  (`/Game/Blueprints/UI/EventUI.SetEvent` _asevent_ui Descriptor Event))

(event `self.DisplayWarning`
  (params (Warning :type String))
  (bind _aswarning_ui (cast `/Game/Blueprints/UI/WarningUI` (`self.WarningUIInstance`)))
  (`/Game/Blueprints/UI/WarningUI.Run Warning Animation` _aswarning_ui Warning))

(event `self.DisplayLaws`
  (bind _asparliament_ui (cast `/Game/Blueprints/UI/Parliament/ParliamentUI` (`self.ParliamentUIInstance`)))
  (`/Game/Blueprints/UI/Parliament/ParliamentUI.DisplayBills&Laws` _asparliament_ui))

(event `self.DisplayNewBill`
  (bind _asparliament_ui (cast `/Game/Blueprints/UI/Parliament/ParliamentUI` (`self.ParliamentUIInstance`)))
  (`/Game/Blueprints/UI/Parliament/ParliamentUI.DisplayProposition` _asparliament_ui))

(event `self.RefreshRepresentatives`
  (bind _asparliament_ui (cast `/Game/Blueprints/UI/Parliament/ParliamentUI` (`self.ParliamentUIInstance`)))
  (`/Game/Blueprints/UI/Parliament/ParliamentUI.DisplayRepresentatives` _asparliament_ui))

(event `self.UpdateRepresentative`
  (params (Index :type Integer))
  (bind _asparliament_ui (cast `/Game/Blueprints/UI/Parliament/ParliamentUI` (`self.ParliamentUIInstance`)))
  (`/Game/Blueprints/UI/Parliament/ParliamentUI.UpdateRepresentative` _asparliament_ui Index))

(event `self.LawPassed`
  (params (bPassed :type Boolean) (Description :type String) (For :type Integer) (Against :type Integer))
  (bind _aslaw_passed_ui (cast `/Game/Blueprints/UI/Parliament/LawPassedUI` (`self.LawPassedUIInstance`)))
  (`/Game/Blueprints/UI/Parliament/LawPassedUI.LawPassed` _aslaw_passed_ui bPassed Description For Against))

(event `self.UpdateMapSeed`
  (params (Seed :type String))
  (bind _asmap_ui (cast `/Game/Blueprints/UI/Map/MapUI` (`Grid.MapUIInstance` (`self.Grid`))))
  (`/Game/Blueprints/UI/Map/MapUI.UpdateSeed` _asmap_ui Seed))

(event `self.UpdateMapAIUI`
  (bind _asmap_ui (cast `/Game/Blueprints/UI/Map/MapUI` (`Grid.MapUIInstance` (`self.Grid`))))
  (`/Game/Blueprints/UI/Map/MapUI.SetAINum` _asmap_ui))

(event `self.UpdateResolutionText`
  (bind _assettings_ui (cast `/Game/Blueprints/UI/Menus/SettingsUI` (`self.SettingsUIInstance`)))
  (`/Game/Blueprints/UI/Menus/SettingsUI.SetResolution` _assettings_ui))

(event `self.SetFactionsInDiplomacyUI`
  (bind _asconquest_ui (cast `/Game/Blueprints/UI/Conquest/ConquestUI` (`self.DiplomacyUIInstance`)))
  (`/Game/Blueprints/UI/Conquest/ConquestUI.SetFactionsInDiplomacy` _asconquest_ui))

(event `self.UpdateFactionIcons`
  (params (Index :type Integer))
  (bind _asconquest_ui (cast `/Game/Blueprints/UI/Conquest/ConquestUI` (`self.DiplomacyUIInstance`)))
  (bind _returnvalue (`PanelWidget.GetChildAt` (`/Game/Blueprints/UI/Conquest/ConquestUI.FactionBtnContainer` _asconquest_ui) Index))
  (if (`KismetSystemLibrary.IsValid` _returnvalue)
    (bind _asfaction_btn (cast `/Game/Blueprints/UI/Conquest/FactionBtn` _returnvalue))
    (`/Game/Blueprints/UI/Conquest/FactionBtn.UpdateFactionIcons` _asfaction_btn)))

(event `self.UpdateFactionHappiness`
  (bind _asconquest_ui (cast `/Game/Blueprints/UI/Conquest/ConquestUI` (`self.DiplomacyUIInstance`)))
  (if (`Widget.IsVisible` (`/Game/Blueprints/UI/Conquest/ConquestUI.DiplomacyContainer` _asconquest_ui))
    (`/Game/Blueprints/UI/Conquest/ConquestUI.PopulateHappiness` _asconquest_ui)))

(event `self.RemoveFactionBtn`
  (params (Index :type Integer))
  (bind _asconquest_ui (cast `/Game/Blueprints/UI/Conquest/ConquestUI` (`self.DiplomacyUIInstance`)))
  (`PanelWidget.RemoveChildAt` (`/Game/Blueprints/UI/Conquest/ConquestUI.FactionBtnContainer` _asconquest_ui) Index))

(event `self.NotifyConquestEvent`
  (params (Message :type String) (FactionName :type String) (bChoice :type Boolean))
  (bind _asconquest_notification_ui (cast `/Game/Blueprints/UI/Conquest/ConquestNotificationUI` (`self.DiplomacyNotifyUIInstance`)))
  (`/Game/Blueprints/UI/Conquest/ConquestNotificationUI.Notify` _asconquest_notification_ui Message FactionName bChoice))

(event `self.DisplayNotifyLog`
  (params (Actor :type "Actor Object Reference") (Type :type String) (Message :type String) (IslandName :type String))
  (bind _aslog_ui (cast `/Game/Blueprints/UI/LogUI` (`self.LogUIInstance`)))
  (`/Game/Blueprints/UI/LogUI.AddToLog` _aslog_ui Actor Type IslandName Message))

(event `self.ClearLog`
  (bind _aslog_ui (cast `/Game/Blueprints/UI/LogUI` (`self.LogUIInstance`)))
  (`/Game/Blueprints/UI/LogUI.ClearLog` _aslog_ui))

(event `self.UpdateMapSpecialBuildings`
  (bind _asmap_ui (cast `/Game/Blueprints/UI/Map/MapUI` (`Grid.MapUIInstance` (`self.Grid`))))
  (`/Game/Blueprints/UI/Map/MapUI.UpdateSpecialBuildings` _asmap_ui))

(event `self.UpdateLoadingText`
  (params (Message :type String))
  (bind _asload_ui (cast `/Game/Blueprints/UI/Map/LoadUI` (`Grid.LoadUIInstance` (`self.Grid`))))
  (`/Game/Blueprints/UI/Map/LoadUI.SetLoadingText` _asload_ui Message))

(event `self.UpdateArmyCountUI`
  (params (Index :type Integer) (Amount :type Integer))
  (bind _asmain_ui (cast `/Game/Blueprints/UI/MainUI` (`self.BuildUIInstance`)))
  (`/Game/Blueprints/UI/Conquest/Army/ArmyUI.UpdateArmyCount` (`/Game/Blueprints/UI/MainUI.ArmyUI` _asmain_ui) Index Amount))

(event `self.UpdateWaveUI`
  (params (Days :type String) (Percentage :type "Float (single-precision)"))
  (bind _asmain_ui (cast `/Game/Blueprints/UI/MainUI` (`self.BuildUIInstance`)))
  (`/Game/Blueprints/UI/MainUI.SetWaveUI` _asmain_ui Days Percentage))

(event `self.InitialiseInfoDisplay`
  (bind _asmain_info_ui (cast `/Game/Blueprints/UI/Info/MainInfoUI` (`self.InfoUIInstance`)))
  (`/Game/Blueprints/UI/Info/MainInfoUI.InitialiseCitizenInfo` _asmain_info_ui))

(event `self.ClearInfoDisplay`
  (bind _asmain_info_ui (cast `/Game/Blueprints/UI/Info/MainInfoUI` (`self.InfoUIInstance`)))
  (`/Game/Blueprints/UI/Info/MainInfoUI.ClearCitizenInfo` _asmain_info_ui)
  (`/Game/Blueprints/UI/Info/MainInfoUI.ClearBuildingInfo` _asmain_info_ui))

(event `self.UpdateCitizenInfoDisplay`
  (params (Type :type "EInfoUpdate Enum" :default "Party") (NameCount :type "Map of String to Integer (by ref)") (LeaderName :type String))
  (bind _asmain_info_ui (cast `/Game/Blueprints/UI/Info/MainInfoUI` (`self.InfoUIInstance`)))
  (`/Game/Blueprints/UI/Info/MainInfoUI.UpdateCitizenInfo` _asmain_info_ui Type NameCount LeaderName))

(event `self.UpdateBuildingInfoDisplay`
  (params (Building :type "Building Object Reference") (bAdd :type Boolean))
  (bind _asmain_info_ui (cast `/Game/Blueprints/UI/Info/MainInfoUI` (`self.InfoUIInstance`)))
  (`/Game/Blueprints/UI/Info/MainInfoUI.UpdateBuildingInfo` _asmain_info_ui Building bAdd))

(event `self.UpdateBuildingMinMaxAmountDisplay`
  (params (Building :type "Building Object Reference"))
  (bind _asmain_info_ui (cast `/Game/Blueprints/UI/Info/MainInfoUI` (`self.InfoUIInstance`)))
  (`/Game/Blueprints/UI/Info/MainInfoUI.UpdateBuildingMinMaxAmount` _asmain_info_ui Building))

(event `self.UpdateBuildingOccupantsDisplay`
  (params (Building :type "Building Object Reference"))
  (bind _asmain_info_ui (cast `/Game/Blueprints/UI/Info/MainInfoUI` (`self.InfoUIInstance`)))
  (`/Game/Blueprints/UI/Info/MainInfoUI.UpdateBuildingOccupants` _asmain_info_ui Building))

(event `self.UpdateEventInfoDisplay`
  (bind _asmain_info_ui (cast `/Game/Blueprints/UI/Info/MainInfoUI` (`self.InfoUIInstance`)))
  (`/Game/Blueprints/UI/Info/MainInfoUI.DisplayEvents` _asmain_info_ui))

(event `self.UpdateVisitors`
  (params (Building :type "Building Object Reference") (Citizen :type "Citizen Object Reference") (bAdd :type Boolean))
  (bind _asvisitors_list_ui (cast `/Game/Blueprints/UI/Interactions/InteractUI-Sections/Building/Visitors/VisitorsListUI` (`self.VisitorsUIInstance`)))
  (`/Game/Blueprints/UI/Interactions/InteractUI-Sections/Building/Visitors/VisitorsListUI.UpdateVisitor` _asvisitors_list_ui Building Citizen bAdd))

(event `self.UnlockAchievement`
  (params (Name :type String))
  (bind _returnvalue (`GameplayStatics.GetPlayerController` 0))
  (`AchievementQueryCallbackProxy.CacheAchievements` _returnvalue
    (:`OnSuccess`
      (`AchievementWriteCallbackProxy.WriteProgress` _returnvalue Name))))

(fn `UserConstructionScript`)